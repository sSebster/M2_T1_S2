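; Player controller for arcade-style control of the BP_Puppet actor found in the level.
; On BeginPlay it adds the IMC_Arcade Enhanced Input mapping context and caches the puppet.
; Holding a limb button (arm, hand, leg or foot, either side) activates that limb's NS effect and adds its stable mesh to SelectedBones; releasing undoes both.
; Joystick input is forwarded to the puppet's ReceiveArcadeInput as a 2D vector.
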(event Input|EnhancedActionEvents|EnhancedInputActionIA_MoveJoyStick
  (params (ActionValue :type Vector%202D%20Structure) (ElapsedSeconds :type Float%20%28double-precision%29) (TriggeredSeconds :type Float%20%28double-precision%29) (InputAction :type Input%20Action%20Object%20Reference :default "/Game/Capture/InputMapping/IA_MoveJoyStick.IA_MoveJoyStick"))
  (Default|ReceiveArcadeInput (Variables|Default|GetPuppet) (Math|Conversions|ToVector(Vector2D) ActionValue)))

(event Input|EnhancedActionEvents|EnhancedInputActionIA_SelectRightArm
  (params (ActionValue :type Boolean) (ElapsedSeconds :type Float%20%28double-precision%29) (TriggeredSeconds :type Float%20%28double-precision%29) (InputAction :type Input%20Action%20Object%20Reference :default "/Game/Capture/InputMapping/IA_SelectRightArm.IA_SelectRightArm"))
  (bind _puppet (Variables|Default|GetPuppet))
  (bind _puppet_2 (Variables|Default|GetPuppet))
  (bind _selectedbones (Variables|/Game/Capture/BP_Puppet.BP_Puppet_C|GetSelectedBones _puppet))
  (bind _rightarmstablemesh (Variables|/Game/Capture/BP_Puppet.BP_Puppet_C|GetRightArmStableMesh _puppet))
  (bind _ns_rforearm (Variables|/Game/Capture/BP_Puppet.BP_Puppet_C|GetNS_RForeArm _puppet_2))
  (:Started
    (Components|Activation|Activate _ns_rforearm false)
    (Utilities|Array|Add _selectedbones _rightarmstablemesh))
  (:Completed
    (Components|Activation|Deactivate _ns_rforearm)
    (Utilities|Array|RemoveItem _selectedbones _rightarmstablemesh)))

(event Input|EnhancedActionEvents|EnhancedInputActionIA_SelectLeftArm
  (params (ActionValue :type Boolean) (ElapsedSeconds :type Float%20%28double-precision%29) (TriggeredSeconds :type Float%20%28double-precision%29) (InputAction :type Input%20Action%20Object%20Reference :default "/Game/Capture/InputMapping/IA_SelectLeftArm.IA_SelectLeftArm"))
  (bind _puppet (Variables|Default|GetPuppet))
  (bind _puppet_2 (Variables|Default|GetPuppet))
  (bind _ns_lforearm (Variables|/Game/Capture/BP_Puppet.BP_Puppet_C|GetNS_LForeArm _puppet))
  (bind _leftarmstablemesh (Variables|/Game/Capture/BP_Puppet.BP_Puppet_C|GetLeftArmStableMesh _puppet_2))
  (bind _selectedbones (Variables|/Game/Capture/BP_Puppet.BP_Puppet_C|GetSelectedBones _puppet_2))
  (:Started
    (Components|Activation|Activate _ns_lforearm false)
    (Utilities|Array|Add _selectedbones _leftarmstablemesh))
  (:Completed
    (Components|Activation|Deactivate _ns_lforearm)
    (Utilities|Array|RemoveItem _selectedbones _leftarmstablemesh)))

(event Input|EnhancedActionEvents|EnhancedInputActionIA_SelectLeftHand
  (params (ActionValue :type Boolean) (ElapsedSeconds :type Float%20%28double-precision%29) (TriggeredSeconds :type Float%20%28double-precision%29) (InputAction :type Input%20Action%20Object%20Reference :default "/Game/Capture/InputMapping/IA_SelectLeftHand.IA_SelectLeftHand"))
  (bind _puppet (Variables|Default|GetPuppet))
  (bind _puppet_2 (Variables|Default|GetPuppet))
  (bind _ns_lhand (Variables|/Game/Capture/BP_Puppet.BP_Puppet_C|GetNS_LHand _puppet))
  (bind _lefthandstablemesh (Variables|/Game/Capture/BP_Puppet.BP_Puppet_C|GetLeftHandStableMesh _puppet_2))
  (bind _selectedbones (Variables|/Game/Capture/BP_Puppet.BP_Puppet_C|GetSelectedBones _puppet_2))
  (:Started
    (Components|Activation|Activate _ns_lhand false)
    (Utilities|Array|Add _selectedbones _lefthandstablemesh))
  (:Completed
    (Components|Activation|Deactivate _ns_lhand)
    (Utilities|Array|RemoveItem _selectedbones _lefthandstablemesh)))

(event Input|EnhancedActionEvents|EnhancedInputActionIA_SelectRightHand
  (params (ActionValue :type Boolean) (ElapsedSeconds :type Float%20%28double-precision%29) (TriggeredSeconds :type Float%20%28double-precision%29) (InputAction :type Input%20Action%20Object%20Reference :default "/Game/Capture/InputMapping/IA_SelectRightHand.IA_SelectRightHand"))
  (bind _puppet (Variables|Default|GetPuppet))
  (bind _puppet_2 (Variables|Default|GetPuppet))
  (bind _selectedbones (Variables|/Game/Capture/BP_Puppet.BP_Puppet_C|GetSelectedBones _puppet_2))
  (bind _righthandstablemesh (Variables|/Game/Capture/BP_Puppet.BP_Puppet_C|GetRightHandStableMesh _puppet_2))
  (bind _ns_rhand (Variables|/Game/Capture/BP_Puppet.BP_Puppet_C|GetNS_RHand _puppet))
  (:Started
    (Components|Activation|Activate _ns_rhand false)
    (Utilities|Array|Add _selectedbones _righthandstablemesh))
  (:Completed
    (Components|Activation|Deactivate _ns_rhand)
    (Utilities|Array|RemoveItem _selectedbones _righthandstablemesh)))

(event Input|EnhancedActionEvents|EnhancedInputActionIA_SelectRightLeg
  (params (ActionValue :type Boolean) (ElapsedSeconds :type Float%20%28double-precision%29) (TriggeredSeconds :type Float%20%28double-precision%29) (InputAction :type Input%20Action%20Object%20Reference :default "/Game/Capture/InputMapping/IA_SelectRightLeg.IA_SelectRightLeg"))
  (bind _puppet (Variables|Default|GetPuppet))
  (bind _puppet_2 (Variables|Default|GetPuppet))
  (bind _ns_rleg (Variables|/Game/Capture/BP_Puppet.BP_Puppet_C|GetNS_RLeg _puppet))
  (bind _selectedbones (Variables|/Game/Capture/BP_Puppet.BP_Puppet_C|GetSelectedBones _puppet_2))
  (bind _rightlegstablemesh (Variables|/Game/Capture/BP_Puppet.BP_Puppet_C|GetRightLegStableMesh _puppet_2))
  (:Started
    (Components|Activation|Activate _ns_rleg false)
    (Utilities|Array|Add _selectedbones _rightlegstablemesh))
  (:Completed
    (Components|Activation|Deactivate _ns_rleg)
    (Utilities|Array|RemoveItem _selectedbones _rightlegstablemesh)))

(event Input|EnhancedActionEvents|EnhancedInputActionIA_SelectRightFeet
  (params (ActionValue :type Boolean) (ElapsedSeconds :type Float%20%28double-precision%29) (TriggeredSeconds :type Float%20%28double-precision%29) (InputAction :type Input%20Action%20Object%20Reference :default "/Game/Capture/InputMapping/IA_SelectRightFeet.IA_SelectRightFeet"))
  (bind _puppet (Variables|Default|GetPuppet))
  (bind _puppet_2 (Variables|Default|GetPuppet))
  (bind _ns_rfoot (Variables|/Game/Capture/BP_Puppet.BP_Puppet_C|GetNS_RFoot _puppet))
  (bind _selectedbones (Variables|/Game/Capture/BP_Puppet.BP_Puppet_C|GetSelectedBones _puppet_2))
  (bind _rightfeetstablemesh (Variables|/Game/Capture/BP_Puppet.BP_Puppet_C|GetRightFeetStableMesh _puppet_2))
  (:Started
    (Components|Activation|Activate _ns_rfoot false)
    (Utilities|Array|Add _selectedbones _rightfeetstablemesh))
  (:Completed
    (Components|Activation|Deactivate _ns_rfoot)
    (Utilities|Array|RemoveItem _selectedbones _rightfeetstablemesh)))

(event Input|EnhancedActionEvents|EnhancedInputActionIA_SelectLeftLeg
  (params (ActionValue :type Boolean) (ElapsedSeconds :type Float%20%28double-precision%29) (TriggeredSeconds :type Float%20%28double-precision%29) (InputAction :type Input%20Action%20Object%20Reference :default "/Game/Capture/InputMapping/IA_SelectLeftLeg.IA_SelectLeftLeg"))
  (bind _puppet (Variables|Default|GetPuppet))
  (bind _puppet_2 (Variables|Default|GetPuppet))
  (bind _leftlegstablemesh (Variables|/Game/Capture/BP_Puppet.BP_Puppet_C|GetLeftLegStableMesh _puppet))
  (bind _selectedbones (Variables|/Game/Capture/BP_Puppet.BP_Puppet_C|GetSelectedBones _puppet))
  (bind _ns_lleg (Variables|/Game/Capture/BP_Puppet.BP_Puppet_C|GetNS_LLeg _puppet_2))
  (:Started
    (Components|Activation|Activate _ns_lleg false)
    (Utilities|Array|Add _selectedbones _leftlegstablemesh))
  (:Completed
    (Components|Activation|Deactivate _ns_lleg)
    (Utilities|Array|RemoveItem _selectedbones _leftlegstablemesh)))

(event Input|EnhancedActionEvents|EnhancedInputActionIA_SelectLeftFeet
  (params (ActionValue :type Boolean) (ElapsedSeconds :type Float%20%28double-precision%29) (TriggeredSeconds :type Float%20%28double-precision%29) (InputAction :type Input%20Action%20Object%20Reference :default "/Game/Capture/InputMapping/IA_SelectLeftFeet.IA_SelectLeftFeet"))
  (bind _puppet (Variables|Default|GetPuppet))
  (bind _puppet_2 (Variables|Default|GetPuppet))
  (bind _leftfeetstablemesh (Variables|/Game/Capture/BP_Puppet.BP_Puppet_C|GetLeftFeetStableMesh _puppet))
  (bind _selectedbones (Variables|/Game/Capture/BP_Puppet.BP_Puppet_C|GetSelectedBones _puppet))
  (bind _ns_lfoot (Variables|/Game/Capture/BP_Puppet.BP_Puppet_C|GetNS_LFoot _puppet_2))
  (:Started
    (Components|Activation|Activate _ns_lfoot false)
    (Utilities|Array|Add _selectedbones _leftfeetstablemesh))
  (:Completed
    (Components|Activation|Deactivate _ns_lfoot)
    (Utilities|Array|RemoveItem _selectedbones _leftfeetstablemesh)))

(event EventBeginPlay
  (bind _asplayer_controller (Utilities|Casting|CastToPlayerController (Game|GetPlayerController 0)))
  (Input|AddMappingContext (PlayerController|LocalPlayerSubsystems|GetEnhancedInputLocalPlayerSubsystem _asplayer_controller) "/Game/Capture/InputMapping/IMC_Arcade.IMC_Arcade" 0 "(bIgnoreAllPressedKeysUntilRelease=True,bForceImmediately=False,bNotifyUserSettings=False)")
  (Development|PrintString "mapping contexte added")
  (bind _returnvalue (Actor|GetActorOfClass "/Game/Capture/BP_Puppet.BP_Puppet_C"))
  (Variables|Default|SetPuppet _returnvalue))

(fn ConstructionScript)