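; BP_Puppet is a puppet actor whose selected static mesh "bones" are moved by arcade input.
; BeginPlay caches each static mesh component's world location as its rest position.
; ReceiveArcadeInput converts the 2D input into a normalized X/Z step and offsets each selected bone only while it stays within MaxBonesSpacing of that rest position.
; An older bone-rotation path, with separate handling for legs, is left unconnected.
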(event Custom|ReceiveArcadeInput
  (params (vec2 :type Vector))
  (bind _returnvalue (* vec2 -2.0))
  (bind (_x _y) (Math|Vector|BreakVector _returnvalue))
  (for _array_element (Variables|Default|GetSelectedBones)
    (Variables|Default|SetMovementVector (Math|Vector|Normalize (Math|Vector|MakeVector _y 0.0 (* _x -1.0))))
    (Variables|Default|SetTargetPosition (+ (Variables|Default|GetMovementVector) (Transformation|GetWorldLocation _array_element)))
    (if (< (Math|Vector|VectorLength (- (Variables|Default|GetTargetPosition) (.Value (Utilities|Map|Find (Variables|Default|GetBonesPosMap) _array_element)))) (Variables|Default|GetMaxBonesSpacing))
      (Transformation|AddWorldOffset _array_element (Variables|Default|GetMovementVector) false false))))

(event EventBeginPlay
  (for _array_element (Actor|GetComponentsByClass "/Script/Engine.StaticMeshComponent")
    (Utilities|Map|Add (Variables|Default|GetBonesPosMap) _array_element (Transformation|GetWorldLocation _array_element))))

(event Collision|EventActorBeginOverlap
  (params (OtherActor :type Actor%20Object%20Reference)))

(fn ConstructionScript)